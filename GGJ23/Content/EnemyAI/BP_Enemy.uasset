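; Enemy actor that tracks health, exposes timed attack and hit flags, and handles death and random loot drops.
; Damage lowers Health; at zero it sets the IsEnemyDead blackboard key, then drops loot and destroys itself once after a delay.
; Loot is a one-in-six resource drop, otherwise a one-in-six health drop.
; Roaming, sight-based movement and spawn-point cleanup are disconnected, leaving those events empty.
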(event `self.ReceiveBeginPlay`)

(event `Random Roam`
  ;[1 1 1] Random Roam Logic
)

(event `self.PawnSensing.OnSeePawn`
  (params (Pawn :type "Pawn Object Reference")))

(event `AttackPlayer`
  (set `self.IsAttacking?` true)
  (`KismetSystemLibrary.Delay` 1.0)
  (set `self.IsAttacking?` false))

(event `self.ReceiveDestroyed`)

(event `self.ReceiveAnyDamage`
  (params (Damage :type "Float (single-precision)") (DamageType :type "DamageType Object Reference") (InstigatedBy :type "Controller Object Reference") (DamageCauser :type "Actor Object Reference"))
  (bind _health (`self.Health`))
  (set `self.IsHit?` true)
  (set `self.Health` (- _health Damage))
  (`KismetSystemLibrary.Delay` 1.0)
  (set `self.IsHit?` false)
  (if (<= _health 0.0)
    (`BlackboardComponent.SetValueAsBool` (`AIBlueprintHelperLibrary.GetBlackboard` null) "IsEnemyDead" true)
    (`/Engine/EditorBlueprintResources/StandardMacros.DoOnce` false
      (:`Completed`
        (`self.DropLoot`)
        (`KismetSystemLibrary.Delay` 3.0)
        (`self.K2_DestroyActor`)))))

(event `DropLoot`
  (if (>= (`KismetMathLibrary.RandomIntegerInRange` 0 5) 5)
    (`|SpawnActorFromClass` "/Game/Blueprints/BP_Resources_Drop.BP_Resources_Drop_C" (`SceneComponent.K2_GetComponentToWorld` (`self.CapsuleComponent`)) "AlwaysSpawn" "OverrideRootScale" null null)
    (elif (>= (`KismetMathLibrary.RandomIntegerInRange` 0 5) 5)
      (`|SpawnActorFromClass` "/Game/Blueprints/BP_Health_Drop.BP_Health_Drop_C" (`SceneComponent.K2_GetComponentToWorld` (`self.CapsuleComponent`)) "AlwaysSpawn" "OverrideRootScale" null null))))

(fn `UserConstructionScript`)
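; BP_Enemy is an AI enemy that roams at random and pursues pawns it sees.
; Roaming waits a random delay, moves to a reachable nearby point and repeats when the move succeeds.
; PawnSensing sightings start a chase, with a retriggerable delay restarting roaming a few seconds after the last sighting.
; On destruction it removes itself from its spawn point's active enemy list.
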(event `Random Roam`
  ;[1 1 1] Random Roam Logic
  (`KismetSystemLibrary.Delay` (`KismetMathLibrary.RandomFloatInRange` 1.0 3.0))
  (`|AIMoveTo` self (`NavigationSystemV1.K2_GetRandomReachablePointInRadius` (`self.K2_GetActorLocation`) 1000.0 null null) null
    (:`OnSuccess`
      (`self.Random Roam`))))

(event `self.ReceiveBeginPlay`
  ;[1 1 1] Random Roam Logic
  (`self.Random Roam`))

(event `self.PawnSensing.OnSeePawn`
  (params (Pawn :type "Pawn Object Reference"))
  (`|ExecutionSequence`
    (:`then_0`
      (`|AIMoveTo` self (0.0 0.0 0.0) Pawn))
    (:`then_1`
      (`KismetSystemLibrary.RetriggerableDelay` 3.0)
      (`self.Random Roam`))))

(event `self.ReceiveDestroyed`
  (`KismetArrayLibrary.Array_RemoveItem` (`/Game/BP_SpawnPoint.ActiveEnemy` (`self.SpawnPoint`)) self))

(fn `UserConstructionScript`)
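; Boss spawn actor that places one BP_Enemy at a random spot within its Box when play begins.
; SpawnEnemy line-traces down from high above the box against WorldStatic and spawns the enemy slightly above the hit, without checking that it hit.
; ReSpawnEnemy spawns another if IsRespawnNode is set and ActiveEnemy is below SpawnAmount.
; The controller setup and ActiveEnemy registration are disconnected, so spawns here never join that count.
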(event `self.ReceiveBeginPlay`
  (`self.SpawnEnemy`))

(fn `ReSpawnEnemy`
  (if (and (< (`KismetArrayLibrary.Array_Length` (`self.ActiveEnemy`)) (`self.SpawnAmount`)) (`self.isRespawnNode`))
    (`self.SpawnEnemy`)))

(fn `SpawnEnemy`
  (bind (_origin _boxextent) (`KismetSystemLibrary.GetComponentBounds` (`self.Box`)))
  (bind _returnvalue (`KismetMathLibrary.MakeVector` (.x (`KismetMathLibrary.RandomPointInBoundingBox` _origin _boxextent)) (.y (`KismetMathLibrary.RandomPointInBoundingBox` _origin _boxextent)) (+ (.z (`KismetMathLibrary.RandomPointInBoundingBox` _origin _boxextent)) 10000.0)))
  (bind _outhit (`KismetSystemLibrary.LineTraceSingleForObjects` _returnvalue (+ _returnvalue (* (* (`self.GetActorUpVector`) -1.0) 15000.0)) (`|MakeArray` "ObjectTypeQuery1" :!type "EObjectTypeQuery Enum")))
  (bind _returnvalue_2 (`|SpawnActorFromClass` "/Game/EnemyAI/BP_Enemy.BP_Enemy_C" (`KismetMathLibrary.MakeTransform` (`KismetMathLibrary.MakeVector` (.x (`.Location` (`GameplayStatics.BreakHitResult` _outhit))) (.y (`.Location` (`GameplayStatics.BreakHitResult` _outhit))) (+ (.z (`.Location` (`GameplayStatics.BreakHitResult` _outhit))) 100.0)) (`KismetMathLibrary.MakeRotator` 0.0 0.0 (`KismetMathLibrary.RandomFloat`))) "AdjustIfPossibleButAlwaysSpawn" "OverrideRootScale" null null)))

(fn `UserConstructionScript`)
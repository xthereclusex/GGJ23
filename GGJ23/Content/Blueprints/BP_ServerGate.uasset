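; BP_ServerGate is a two-door gate that opens on command and shows a text label while the player character is inside its trigger box.
; Box overlap begin and end events only toggle the TextRender's visibility.
; A separate OpenDoor custom event starts a timeline for each door, interpolating its relative location and rotation between start and end transforms held in struct variables.
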(event `self.Box.OnComponentBeginOverlap`
  (params (OverlappedComponent :type "PrimitiveComponent Object Reference") (OtherActor :type "Actor Object Reference") (OtherComp :type "PrimitiveComponent Object Reference") (OtherBodyIndex :type Integer) (bFromSweep :type Boolean) (SweepResult :type "HitResult Structure (by ref)"))
  ;[1 1 1] Set Visibility to Render Text when overlapping with Player Character
  (if (== OtherActor null)
    (`SceneComponent.SetVisibility` (`self.TextRender`) true false)))

(event `self.Box.OnComponentEndOverlap`
  (params (OverlappedComponent :type "PrimitiveComponent Object Reference") (OtherActor :type "Actor Object Reference") (OtherComp :type "PrimitiveComponent Object Reference") (OtherBodyIndex :type Integer))
  ;[1 1 1] Set Visibility to Render Text when overlapping with Player Character
  (if (== OtherActor null)
    (`SceneComponent.SetVisibility` (`self.TextRender`) false false)))

(event `OpenDoor`
  (bind (_leftdoorstructend_doorlocation _leftdoorstructend_doorrotation) (break `/Game/Blueprints/Struct_ServerGates` (`self.LeftDoorStructEnd`)))
  (bind (_rightdoorstructstart_doorlocation _rightdoorstructstart_doorrotation) (break `/Game/Blueprints/Struct_ServerGates` (`self.RightDoorStructStart`)))
  (bind (_rightdoorstructend_doorlocation _rightdoorstructend_doorrotation) (break `/Game/Blueprints/Struct_ServerGates` (`self.RightDoorStructEnd`)))
  (bind (_leftdoorstructstart_doorlocation _leftdoorstructstart_doorrotation) (break `/Game/Blueprints/Struct_ServerGates` (`self.LeftDoorStructStart`)))
  ;[1 1 1] Custom Event to Open the Gate
  (`|ExecutionSequence`
    (:`then_0`
      (bind (_direction _alpha) (`Timeline|LeftDoorTL` :!via `PlayFromStart`)
        (:`Update`
          (`SceneComponent.K2_SetRelativeLocationAndRotation` (`self.LeftDoor`) (`KismetMathLibrary.VLerp` _leftdoorstructstart_doorlocation _leftdoorstructend_doorlocation _alpha) (`KismetMathLibrary.RLerp` _leftdoorstructstart_doorrotation _leftdoorstructend_doorrotation _alpha) false false))))
    (:`then_1`
      (bind (_direction_2 _alpha_2) (`Timeline|RightDoorTL` :!via `PlayFromStart`)
        (:`Update`
          (`SceneComponent.K2_SetRelativeLocationAndRotation` (`self.RightDoor`) (`KismetMathLibrary.VLerp` _rightdoorstructstart_doorlocation _rightdoorstructend_doorlocation _alpha_2) (`KismetMathLibrary.RLerp` _rightdoorstructstart_doorrotation _rightdoorstructend_doorrotation _alpha_2) false false))))))

(fn `UserConstructionScript`)
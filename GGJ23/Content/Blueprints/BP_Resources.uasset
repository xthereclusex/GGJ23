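; BP_Resources is a gatherable resource pickup that adds to the player's resource count.
; Overlap with Sphere1 shows a TextRender label and end overlap hides it, with no check on which actor overlaps.
; The Interact event casts player 0's character to SP_Player, adds ResourcesGathered to its Resource, then destroys the pickup after a short delay.
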(event `self.Sphere1.OnComponentBeginOverlap`
  (params (OverlappedComponent :type "PrimitiveComponent Object Reference") (OtherActor :type "Actor Object Reference") (OtherComp :type "PrimitiveComponent Object Reference") (OtherBodyIndex :type Integer) (bFromSweep :type Boolean) (SweepResult :type "HitResult Structure (by ref)"))
  ;[1 1 1] Overalps
  (`SceneComponent.SetVisibility` (`self.TextRender`) true false))

(event `self.Sphere1.OnComponentEndOverlap`
  (params (OverlappedComponent :type "PrimitiveComponent Object Reference") (OtherActor :type "Actor Object Reference") (OtherComp :type "PrimitiveComponent Object Reference") (OtherBodyIndex :type Integer))
  ;[1 1 1] Overalps
  (`SceneComponent.SetVisibility` (`self.TextRender`) false false))

(event `/Game/Blueprints/BPI_Interactable.Interact`
  ;[1 1 1] Interact
  (bind _assp_player (cast `/Game/SP_Player` (`GameplayStatics.GetPlayerCharacter` 0)))
  (set `/Game/SP_Player.Resource` (+ (`/Game/SP_Player.Resource` _assp_player) (`self.ResourcesGathered`)) _assp_player)
  (`KismetSystemLibrary.Delay` 0.2)
  (`self.K2_DestroyActor`))

(fn `UserConstructionScript`)
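; Homing rocket projectile whose events launch it along the player's forward vector, play travel and explosion sounds, and deal damage before destroying itself on hit.
; A Lock on Target event enables ProjectileMovement homing toward the component returned by FindHomingTarget.
; Homing is unfinished: the closest "Homing"-tagged actor search is disconnected, leaving FindHomingTarget empty, and the repeating lock-on calls never run.
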(event `ShootLocation`
  ;[1 1 1] Shoot Location
  (bind _assp_player (cast `/Game/SP_Player` (`GameplayStatics.GetPlayerCharacter` 0)))
  (set `MovementComponent.Velocity` (* (`self.GetActorForwardVector` _assp_player) 2000.0) (`self.ProjectileMovement`)))

(event `self.ReceiveHit`
  (params (MyComp :type "PrimitiveComponent Object Reference") (Other :type "Actor Object Reference") (OtherComp :type "PrimitiveComponent Object Reference") (bSelfMoved :type Boolean) (HitLocation :type "Vector Structure") (HitNormal :type "Vector Structure") (NormalImpulse :type "Vector Structure") (Hit :type "HitResult Structure (by ref)"))
  ;[1 1 1] Hit
  (`GameplayStatics.PlaySound2D` "/Game/Audio/Robot/Weapons/Rocket/Rocket_Explode_01.Rocket_Explode_01" 1.0 1.0 0.0 null null)
  (`GameplayStatics.ApplyDamage` Other 20.0 null self)
  (`self.K2_DestroyActor`))

(event `Lock on target`
  (bind _projectilemovement (`self.ProjectileMovement`))
  ;[1 1 1] Lock on target
  (bind _homing_target (`self.Find Homing Target`))
  (set `ProjectileMovementComponent.HomingTargetComponent` _homing_target _projectilemovement)
  (set `ProjectileMovementComponent.bIsHomingProjectile` true _projectilemovement))

(event `self.ReceiveBeginPlay`
  (`GameplayStatics.PlaySound2D` "/Game/Audio/Robot/Weapons/Rocket/Rocket_Travel_Loop_01.Rocket_Travel_Loop_01" 1.0 1.0 0.0 null null))

(fn `Find Homing Target`
  (returns (`Homing Target` :type "SceneComponent Object Reference")))

(fn `UserConstructionScript`)